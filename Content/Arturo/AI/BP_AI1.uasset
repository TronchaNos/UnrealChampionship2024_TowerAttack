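; BP_AI1 is an AI character prototype for random wandering, but the wandering is currently disconnected and never starts.
; BeginPlay only disables mesh physics and stops movement.
; RandomMovement loops three times over async AIMoveTo calls to reachable points near the character, printing debug text and re-calling itself after a delay on success.
; Its branch to RagdollDeath is unreachable because the index never hits 3, and that event is empty.
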(event Custom|RandomMovement
  (for _index (range 0 2)
    (AI|AIMoveTo self (.RandomLocation (AI|Navigation|GetRandomReachablePointinRadius (Transformation|GetActorLocation) 1.5e+03 0 0)) 0 5e+01 false
      (:OnSuccess
        (Development|PrintString (Utilities|String|ToString(Integer) _index) true true "(R=1.000000,G=0.000000,B=0.102800,A=1.000000)" 6.0)
        (Utilities|FlowControl|Delay 1.0)
        (if (!= _index 3)
          (CallFunction|RandomMovement)
          (else
            (CallFunction|RagdollDeath)))
        (Development|PrintString (Utilities|String|ToString(Integer) _index) true true "(R=0.000000,G=0.660000,B=1.000000,A=1.000000)" 6.0)))))

(event Custom|RagdollDeath)

(event EventBeginPlay
  (Physics|SetSimulatePhysics (Variables|Character|GetMesh) false)
  (Components|Movement|StopMovementImmediately (Variables|Character|GetCharacterMovement)))

(event Input|KeyboardEvents|DebugKey2
  (params (Key :type Key%20Structure :default "None") (ActionValue :type Input%20Action%20Value%20Structure)))

(fn ConstructionScript)