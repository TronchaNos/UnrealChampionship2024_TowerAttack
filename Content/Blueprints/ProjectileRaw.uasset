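; Physics projectile actor that launches itself in the YZ plane and destroys itself once it comes to rest or outlives its lifetime.
; BeginPlay applies a force to Sphere1 from Direction times Impulse, mapping X to world Y and negated Y to Z.
; Tick uses a Delay to step roughly one-second timers, resetting the rest timer while moving.
; The stopped check compares signed Y and Z velocities, so negative velocities also count as stopped.
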(event EventBeginPlay
  (bind _direction (Variables|Default|GetDirection))
  (bind _impulse (Variables|Default|GetImpulse))
  (bind _returnvalue (* _direction _impulse))
  (bind (_x _y) (Math|Vector2D|BreakVector2D _returnvalue))
  (Physics|AddForce (Variables|Default|GetSphere1) (Math|Vector|MakeVector 0.0 _x (* _y -1.0)) "None" false))

(event Collision|EventActorBeginOverlap
  (params (OtherActor :type Actor%20Object%20Reference)))

(event EventTick
  (params (DeltaSeconds :type Float%20%28single-precision%29))
  (bind _sphere1 (Variables|Default|GetSphere1))
  (bind _returnvalue (Transformation|GetComponentVelocity _sphere1))
  (Variables|Default|SetIsStopped? (and (<= (.y _returnvalue) 1.0) (<= (.z _returnvalue) 1.0)))
  (Utilities|FlowControl|Delay 1.0)
  (Variables|Default|Settimer (+ (Variables|Default|Gettimer) 1.0))
  (Variables|Default|SetRealTime (+ (Variables|Default|GetRealTime) 1.0))
  (Utilities|FlowControl|Sequence
    (:then_0
      (if (not (Variables|Default|GetIsStopped?))
        (Variables|Default|Settimer 0.0)))
    (:then_1
      (if (or (and (Variables|Default|GetIsStopped?) (>= (Variables|Default|Gettimer) (Variables|Default|GetmaxTimer))) (>= (Variables|Default|GetRealTime) 4e+01))
        (Actor|DestroyActor)))))

(fn ConstructionScript)