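; Explosive projectile actor that detonates once when its hit sphere strikes something.
; The hit spawns explosion particles and a NewBlueprint actor (using the sphere's relative transform), fires a RadialForce impulse, removes both spheres, then destroys itself after a delay.
; A delayed Tick counter acts as a rough lifetime, firing the impulse and destroying the projectile on timeout without effects.
; The construction script sets the impulse limit.
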(event OnComponentHit(Sphere1)
  (params (HitComponent :type Primitive%20Component%20Object%20Reference) (OtherActor :type Actor%20Object%20Reference) (OtherComp :type Primitive%20Component%20Object%20Reference) (NormalImpulse :type Vector :default "0, 0, 0") (Hit :type Hit%20Result%20Structure%20%28by%20ref%29))
  (Utilities|FlowControl|DoOnce false
    (:Completed
      (Effects|SpawnEmitteratLocation "/Game/StarterContent/Particles/P_Explosion.P_Explosion" (Transformation|GetWorldLocation (Variables|Default|GetSphere1)) "0, 0, 0" "2.000000,2.000000,2.000000")
      (Game|SpawnActorfromClass "/Game/Blueprints/NewBlueprint.NewBlueprint_C" (Transformation|GetRelativeTransform (Variables|Default|GetSphere1)) "Undefined" "MultiplyWithRoot" 0 3e+02 0)
      (Class|RadialForceComponent|FireImpulse (Variables|Default|GetRadialForce))
      (Components|DestroyComponent (Variables|Default|GetSphere))
      (Components|DestroyComponent (Variables|Default|GetSphere1))
      (Utilities|FlowControl|Delay 2.0)
      (Actor|DestroyActor))))

(event OnComponentBeginOverlap(Sphere1)
  (params (OverlappedComponent :type Primitive%20Component%20Object%20Reference) (OtherActor :type Actor%20Object%20Reference) (OtherComp :type Primitive%20Component%20Object%20Reference) (OtherBodyIndex :type Integer) (bFromSweep :type Boolean) (SweepResult :type Hit%20Result%20Structure%20%28by%20ref%29)))

(event EventBeginPlay
  (|CallParentFunction))

(event Collision|EventActorBeginOverlap
  (params (OtherActor :type Actor%20Object%20Reference))
  (|CallParentFunction OtherActor) ; This node is disabled and will not be called.\nDrag off pins to build functionality.
)

(event EventTick
  (params (DeltaSeconds :type Float%20%28single-precision%29))
  (Utilities|FlowControl|Delay 1.0)
  (Variables|Default|SetRealTime (+ (Variables|Default|GetRealTime) 1.0))
  (Utilities|FlowControl|Sequence
    (:then_0
      (if (Variables|Default|GetIsStopped?)
        _))
    (:then_1
      (if (>= (Variables|Default|GetRealTime) 4e+01)
        (Class|RadialForceComponent|FireImpulse (Variables|Default|GetRadialForce))
        (Actor|DestroyActor)))))

(fn ConstructionScript
  (|CallParentFunction)
  (Variables|Default|Setimpulse%20limit 2e+05))