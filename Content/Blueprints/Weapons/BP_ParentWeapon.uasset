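; BP_ParentWeapon is a parent weapon Blueprint that fires a projectile and can be outlined.
; LaunchBola plays a Niagara explosion effect at ExplotionSpawner, then after a short delay spawns ProjectileClass at the Box transform, passing it Impulse and Direction.
; SetOutline toggles custom depth rendering on the SMBase mesh for outlining.
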(event Custom|Set%20Outline
  (params (Outline? :type Boolean))
  (Rendering|SetRenderCustomDepth (Variables|Default|GetSM_Base) Outline?))

(event Custom|Launch%20Bola
  (params (Impulse :type Float%20%28double-precision%29) (Direction :type Vector%202D%20Structure))
  (bind _box (Variables|Default|GetBox))
  (bind _explotionspawner (Variables|Default|GetExplotionSpawner))
  (bind _returnvalue (Transformation|GetWorldTransform _box))
  (Niagara|SpawnSystematLocation "/Game/Blueprints/NG_Explotion.NG_Explotion" (Transformation|GetWorldLocation _explotionspawner) (Transformation|GetWorldRotation _explotionspawner))
  (Utilities|FlowControl|Delay 0.1)
  (Game|SpawnActorfromClass (Variables|Default|GetProjectileClass) (Math|Transform|MakeTransform (Math|Vector|MakeVector (.x (.location _returnvalue)) (.y (.location _returnvalue)) (.z (.location _returnvalue))) (.rotation _returnvalue) (.scale _returnvalue)) "AdjustIfPossibleButAlwaysSpawn" "MultiplyWithRoot" 0 Impulse Direction false 0))

(event EventBeginPlay)

(event Collision|EventActorBeginOverlap
  (params (OtherActor :type Actor%20Object%20Reference)))

(event EventTick
  (params (DeltaSeconds :type Float%20%28single-precision%29)))

(fn ConstructionScript)