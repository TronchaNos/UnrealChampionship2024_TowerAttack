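; Projectile actor that launches along a 2D direction in the YZ plane and destroys itself after coming to rest.
; The construction script sets ProjectileMovement speed from Impulse and velocity from Direction, with its vertical component inverted.
; Tick uses a one-second Delay to advance a timer, resetting it while moving and destroying at MaxTimer.
; The stop check compares signed Y and Z velocity, so negative motion also counts as stopped.
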(event OnComponentHit(Sphere)
  (params (HitComponent :type Primitive%20Component%20Object%20Reference) (OtherActor :type Actor%20Object%20Reference) (OtherComp :type Primitive%20Component%20Object%20Reference) (NormalImpulse :type Vector :default "0, 0, 0") (Hit :type Hit%20Result%20Structure%20%28by%20ref%29)))

(event EventBeginPlay
  (Physics|AddImpulse (Variables|Default|GetSphere) "0, 0, 0" "None" false))

(event Collision|EventActorBeginOverlap
  (params (OtherActor :type Actor%20Object%20Reference)))

(event EventTick
  (params (DeltaSeconds :type Float%20%28single-precision%29))
  (bind _projectilemovement (Variables|Default|GetProjectileMovement))
  (bind _velocity (Variables|/Script/Engine.MovementComponent|GetVelocity _projectilemovement))
  (Variables|Default|SetIsStopped? (and (<= (.y _velocity) 1.0) (<= (.z _velocity) 1.0)))
  (Utilities|FlowControl|Delay 1.0)
  (Variables|Default|Settimer (+ (Variables|Default|Gettimer) 1.0))
  (Utilities|FlowControl|Sequence
    (:then_0
      (if (not (Variables|Default|GetIsStopped?))
        (Variables|Default|Settimer 0.0)))
    (:then_1
      (if (and (Variables|Default|GetIsStopped?) (>= (Variables|Default|Gettimer) (Variables|Default|GetmaxTimer)))
        (Actor|DestroyActor)))))

(fn ConstructionScript
  (bind _projectilemovement (Variables|Default|GetProjectileMovement))
  (bind _direction (Variables|Default|GetDirection))
  (bind _impulse (Variables|Default|GetImpulse))
  (bind _returnvalue (* _impulse 1e+01))
  (Variables|/Script/Engine.ProjectileMovementComponent|SetInitialSpeed _projectilemovement _returnvalue)
  (Variables|/Script/Engine.ProjectileMovementComponent|SetMaxSpeed _projectilemovement _returnvalue)
  (Variables|/Script/Engine.MovementComponent|SetVelocity _projectilemovement (Math|Vector|MakeVector 0.0 (.x _direction) (* (.y _direction) -1.0))))