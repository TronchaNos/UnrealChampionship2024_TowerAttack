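; Bridge actor that procedurally builds a physics-driven, breakable hanging bridge from a configurable number of segments.
; The construction script spawns a row of static mesh segments along X, with hidden, non-simulated meshes at both ends serving as anchors.
; Each segment links to the previous one through a physics constraint with a linear break threshold; an angular break setup exists but is unconnected.
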(event EventBeginPlay)

(event Collision|EventActorBeginOverlap
  (params (OtherActor :type Actor%20Object%20Reference)))

(event EventTick
  (params (DeltaSeconds :type Float%20%28single-precision%29)))

(fn ConstructionScript
  (for _index (range 0 (+ (Variables|Default|GetBridgeSegments) 1))
    (Variables|Default|SetIndex _index)
    (Utilities|FlowControl|Sequence
      (:then_0
        (bind _returnvalue (AddComponent|AddStaticMeshComponent false (Math|Transform|MakeTransform (Math|Vector|MakeVector (* _index (Variables|Default|GetMeshOffset)) 0.0 0.0) "0.000000,90.000000,0.000000" "1.000000,1.000000,1.000000")))
        (Utilities|Array|Add (Variables|Default|GetBridgeMeshes) _returnvalue)
        (if (== (Variables|Default|GetIndex) 0)
          (Physics|SetSimulatePhysics _returnvalue false)
          (Transformation|SetRelativeTransform _returnvalue (Math|Transform|MakeTransform (Math|Vector|MakeVector (/ (Variables|Default|GetMeshOffset) 2.0) 0.0 0.0) "0, 0, 0" "0.100000,0.100000,0.075000") false false)
          (Rendering|SetVisibility _returnvalue false false)
          (elif (== (Variables|Default|GetIndex) (+ (Variables|Default|GetBridgeSegments) 1))
            (Physics|SetSimulatePhysics _returnvalue false)
            (Transformation|SetRelativeTransform _returnvalue (Math|Transform|MakeTransform (Math|Vector|MakeVector (- (* (Variables|Default|GetIndex) (Variables|Default|GetMeshOffset)) 1e+02) 0.0 0.0) "0, 0, 0" "0.100000,0.100000,0.075000") false false)
            (Rendering|SetVisibility _returnvalue false false)
            (else
              (Physics|SetSimulatePhysics _returnvalue true)))))
      (:then_1
        (if (> (Variables|Default|GetIndex) 0)
          (bind _returnvalue_2 (AddComponent|AddPhysicsConstraintComponent false (Math|Transform|MakeTransform (Math|Vector|MakeVector (- (* _index (Variables|Default|GetMeshOffset)) (Variables|Default|GetStartPointConstrait)) 0.0 0.0) "-90.000000,0.000000,0.000000" "1.000000,1.000000,1.000000")))
          (Class|PhysicsConstraintComponent|SetConstrainedComponents _returnvalue_2 (Utilities|Array|Get(acopy) (Variables|Default|GetBridgeMeshes) (- (Variables|Default|GetIndex) 1)) "None" (Utilities|Array|Get(acopy) (Variables|Default|GetBridgeMeshes) (Variables|Default|GetIndex)) "None")
          (Class|PhysicsConstraintComponent|SetLinearBreakable _returnvalue_2 true 9e+05))))))