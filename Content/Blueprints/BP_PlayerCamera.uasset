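; Player camera that lets the mouse aim and fire cannons (BP_ParentWeapon) with a slingshot-style drag.
; Each tick it traces under the cursor through PC_Canion to select and outline the hovered cannon.
; IA_Click records the drag start, then Tick rolls the cannon mesh opposite the drag.
; When IA_Click triggers after a long enough drag, LaunchBola fires along that reversed vector with impulse scaled by drag length.
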(event Input|EnhancedActionEvents|EnhancedInputActionIA_Click
  (params (ActionValue :type Boolean) (ElapsedSeconds :type Float%20%28double-precision%29) (TriggeredSeconds :type Float%20%28double-precision%29) (InputAction :type Input%20Action%20Object%20Reference :default "/Game/Blueprints/Control_Mapping/IA_Click.IA_Click"))
  (bind _endmouse (Variables|Default|GetEndMouse))
  (bind (_x _y) (Math|Vector2D|BreakVector2D _endmouse))
  (:Triggered
    ;[1 1 1] if canion was clicked and released launch event
    (if (Variables|Default|GetClickedCanion)
      (if (> (Math|Vector|Distance2D(Vector) _endmouse (Variables|Default|GetStartMouse)) 5e+01)
        (Default|LaunchBola (Variables|Default|GetSelectedCanion) (* (Math|Vector|Distance2D(Vector) _endmouse (Variables|Default|GetStartMouse)) 3e+03) (* (Math|Vector2D|MakeVector2D (- _x (.X (Math|Vector2D|BreakVector2D (Variables|Default|GetStartMouse)))) (- _y (.Y (Math|Vector2D|BreakVector2D (Variables|Default|GetStartMouse))))) -1.0))
        (Default|SetOutline (Variables|Default|GetSelectedCanion) false))))
  (:Started
    ;[1 1 1] If user click on screen
    (Variables|Default|SetClicked true)
    (if (Variables|Default|GetOverCanion)
      ;[1 1 1] Start Preparing Shoot
      (Variables|Default|SetClickedCanion true)
      (bind _returnvalue (Class|WidgetLayoutLibrary|GetMousePositiononViewport))
      (Variables|Default|SetStartMouse _returnvalue)))
  (:Canceled
    ;[1 1 1] Reset variables
    (Variables|Default|SetClickedCanion false :!label _label)
    (Variables|Default|SetClicked false))
  (:Completed
    (goto _label)))

(event EventBeginPlay
  ;[1 1 1] Get level canion references
  (Variables|Default|SetPC_reference (.AsPC%20Canion (Utilities|Casting|CastToPC_Canion (Pawn|GetController)))))

(event Collision|EventActorBeginOverlap
  (params (OtherActor :type Actor%20Object%20Reference)))

(event EventTick
  (params (DeltaSeconds :type Float%20%28single-precision%29))
  (bind _array (Utilities|Array|MakeArray "ObjectTypeQuery2"))
  (bind _pc_reference (Variables|Default|GetPC_reference))
  (bind _startmouse (Variables|Default|GetStartMouse))
  (bind _hitresult (Class|PlayerController|GetHitResultUnderCursorforObjects _pc_reference _array true))
  (bind (_x _y) (Math|Vector2D|BreakVector2D _startmouse))
  (Utilities|FlowControl|Sequence
    (:then_0
      (if (Utilities|ClassIsChildOf (Utilities|GetClass (.hitactor _hitresult)) "/Game/Blueprints/Weapons/BP_ParentWeapon.BP_ParentWeapon_C")
        (Variables|Default|SetOverCanion true)
        (bind _output_get (Variables|Default|SetSelectedCanion (.AsBP%20Parent%20Weapon (Utilities|Casting|CastToBP_ParentWeapon (.hitactor _hitresult)))))
        (Default|SetOutline _output_get true)
        (if (Variables|Default|GetClicked)
          _)
        (else
          (Variables|Default|SetOverCanion false)
          (if (not (Variables|Default|GetClicked))
            (Utilities|IsValid _output_get
              (:Is%20Valid
                (Default|SetOutline _output_get false)))))))
    (:then_1
      ;[1 1 1] calculating shoot
      (if (Variables|Default|GetClickedCanion)
        (bind _returnvalue (Class|WidgetLayoutLibrary|GetMousePositiononViewport))
        (Variables|Default|SetEndMouse _returnvalue)
        (Transformation|SetWorldRotation (Variables|/Game/Blueprints/Weapons/BP_ParentWeapon.BP_ParentWeapon_C|GetSM_Canion (Variables|Default|GetSelectedCanion)) (Math|Rotator|MakeRotator (Class|KismetMathLibrary|DegAtan2 (.Y (Math|Vector2D|BreakVector2D (* (Math|Vector2D|MakeVector2D (- (.X (Math|Vector2D|BreakVector2D (Variables|Default|GetEndMouse))) _x) (- (.Y (Math|Vector2D|BreakVector2D (Variables|Default|GetEndMouse))) _y)) -1.0))) (.X (Math|Vector2D|BreakVector2D (* (Math|Vector2D|MakeVector2D (- (.X (Math|Vector2D|BreakVector2D (Variables|Default|GetEndMouse))) _x) (- (.Y (Math|Vector2D|BreakVector2D (Variables|Default|GetEndMouse))) _y)) -1.0)))) 0.0 0.0) false false)))))

(fn ConstructionScript)